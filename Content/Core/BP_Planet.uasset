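; BP_Planet is a planet actor built on a geometry collection that disappears when it collides with another planet.
; Every tick it moves its collision sphere to the geometry collection's bounds origin, so overlap detection follows the mesh.
; An overlap with another BP_Planet triggers a one-time slowed timeline that scales the collection down, then destroys the actor.
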(event OnComponentBeginOverlap(Sphere)
  (params (OverlappedComponent :type Primitive%20Component%20Object%20Reference) (OtherActor :type Actor%20Object%20Reference) (OtherComp :type Primitive%20Component%20Object%20Reference) (OtherBodyIndex :type Integer) (bFromSweep :type Boolean) (SweepResult :type Hit%20Result%20Structure%20%28by%20ref%29))
  ;[1 1 1] Detectar colisión
  (bind _asbp_planet (Utilities|Casting|CastToBP_Planet OtherActor))
  (if (!= _asbp_planet self)
    (Utilities|FlowControl|DoOnce false
      (:Completed
        (CallFunction|DissapearPlannet)))))

(event Custom|DissapearPlannet
  ;[1 1 1] Desintegrar planeta
  (Components|Timeline|SetPlayRate (Variables|Default|GetTimeline_0) 0.1)
  (bind _newtrack_0 (Timeline|Timeline_0 PlayFromStart)
    (:Update
      (Transformation|SetWorldScale3D (Variables|Default|GetSphere_E56E4C06_GeometryCollection) (Math|Conversions|ToVector(Float) (- 1.0 _newtrack_0))))
    (:Finished
      (Actor|DestroyActor))))

(event Custom|SetSphereTrajectory
  ;[1 1 1] Asignar esfera de colisión
  (Transformation|SetWorldLocation (Variables|Default|GetSphere) (.Origin (Collision|GetComponentBounds (Variables|Default|GetSphere_E56E4C06_GeometryCollection))) false false))

(event EventBeginPlay
  ;[1 1 1] Activar tick
  (Actor|Tick|SetActorTickEnabled true))

(event Collision|EventActorBeginOverlap
  (params (OtherActor :type Actor%20Object%20Reference)))

(event EventTick
  (params (DeltaSeconds :type Float%20%28single-precision%29))
  ;[1 1 1] Eventos del tick
  (CallFunction|SetSphereTrajectory))

(fn ConstructionScript)